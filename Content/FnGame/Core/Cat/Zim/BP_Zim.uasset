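; Zim cat Blueprint that moves in a back-and-forth frolic and announces its spawn with an effect and sound.
; A Delay on Tick paces a Frolic toggle, flipping MoveSpeed between forward and reversed base speed, with the forward phase lasting longer than the backward one.
; OnSpawn activates the spawn effect, plays the Zim sound in 2D, then enables the moving effect after a short delay.
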(event EventOnSpawn
  (Components|Activation|Activate (Variables|Default|GetSpawnEffect) true)
  (Audio|PlaySound2D "/Game/FnGame/Core/Cat/Zim/A_Zim.A_Zim" 1.0 1.0 0.0 0 0)
  (Utilities|FlowControl|Delay 2.0)
  (Components|Activation|Activate (Variables|Default|GetMovingEffect) true))

(event EventTick
  (params (DeltaSeconds :type Float%20%28single-precision%29))
  (bind _basemovespeed (Variables|Default|GetBaseMoveSpeed))
  (Utilities|FlowControl|Delay (Variables|Default|GetDecisionDelay))
  (if (Variables|Default|GetbFrolic)
    (Variables|Default|SetMoveSpeed (* _basemovespeed -1.0))
    (Variables|Default|SetbFrolic false)
    (Variables|Default|SetDecisionDelay 0.5)
    (else
      (Variables|Default|SetMoveSpeed _basemovespeed)
      (Variables|Default|SetbFrolic true)
      (Variables|Default|SetDecisionDelay 1.0))))

(fn ConstructionScript)