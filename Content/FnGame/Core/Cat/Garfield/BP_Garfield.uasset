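; Garfield cat Blueprint that alternates between frolicking at base move speed and standing still.
; Tick feeds a Delay, which ignores calls while pending and so works as a repeating decision timer.
; Each time it completes, it flips the Frolic flag, sets MoveSpeed to base or zero, and sets the next delay, making moving phases longer than pauses.
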(event EventTick
  (params (DeltaSeconds :type Float%20%28single-precision%29))
  (Utilities|FlowControl|Delay (Variables|Default|GetDecisionDelay))
  (if (Variables|Default|GetbFrolic)
    (Variables|Default|SetMoveSpeed 0.0)
    (Variables|Default|SetbFrolic false)
    (Variables|Default|SetDecisionDelay 0.5)
    (else
      (Variables|Default|SetMoveSpeed (Variables|Default|GetBaseMoveSpeed))
      (Variables|Default|SetbFrolic true)
      (Variables|Default|SetDecisionDelay 1.0))))

(fn ConstructionScript)