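; BP_William is a player input Blueprint that requests animal spawns on one of three named paths.
; It caches the BP_MainGM game mode on BeginPlay.
; Releasing input action 1, 2 or 3 calls TryToSpawnAnimal on that game mode with the matching path name, leaving the spawn logic to the game mode.
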(event EventBeginPlay
  (Variables|Default|SetGM (.AsBP%20Main%20GM (Utilities|Casting|CastToBP_MainGM (Game|GetGameMode)))))

(event Input|ActionEvents|InputAction1
  (params (Key :type Key%20Structure))
  (:Released
    (Class|MainGM|TrytoSpawnAnimal (Variables|Default|GetGM) "Path_1")))

(event Input|ActionEvents|InputAction2
  (params (Key :type Key%20Structure))
  (:Released
    (Class|MainGM|TrytoSpawnAnimal (Variables|Default|GetGM) "Path_2")))

(event Input|ActionEvents|InputAction3
  (params (Key :type Key%20Structure))
  (:Released
    (Class|MainGM|TrytoSpawnAnimal (Variables|Default|GetGM) "Path_3")))

(fn ConstructionScript)