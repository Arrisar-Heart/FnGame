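; BP_SuperPawn is a pawn that lets the player spawn animals on one of three named paths using input actions 1, 2 and 3.
; Each input calls SpawnAnimal with a path name, which forwards the request to BP_MainGM, the game mode cached on BeginPlay.
; A successful spawn sets an Overheat flag that blocks further requests for a short delay, while a failed attempt triggers no cooldown.
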(event EventBeginPlay
  (Variables|Default|SetGM (.AsBP%20Main%20GM (Utilities|Casting|CastToBP_MainGM (Game|GetGameMode)))))

(event Input|ActionEvents|InputAction1
  (params (Key :type Key%20Structure :default "None"))
  (:Pressed
    (Utilities|SpawnAnimal "Path_1")))

(event Input|ActionEvents|InputAction2
  (params (Key :type Key%20Structure :default "None"))
  (:Pressed
    (Utilities|SpawnAnimal "Path_2")))

(event Input|ActionEvents|InputAction3
  (params (Key :type Key%20Structure :default "None"))
  (:Pressed
    (Utilities|SpawnAnimal "Path_3")))

(fn ConstructionScript)